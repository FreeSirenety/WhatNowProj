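; MyCharacter2 is an AI-moved character that patrols between two target actors, dies to projectiles and can be caught by a hook shot.
; It starts toward FirstTarget on BeginPlay, and each overlap with one target sends it to the other via SimpleMoveToLocation.
; Overlapping a Projectile destroys it.
; Overlapping an unoccupied HookShot claims that hook, and Tick then snaps the character to the hook's location without sweeping.
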(event EventBeginPlay
  (bind _firsttarget (Variables|Default|GetFirstTarget))
  (if (Utilities|IsValid _firsttarget)
    (AI|Navigation|SimpleMovetoLocation (Pawn|GetController) (Transformation|GetActorLocation _firsttarget))
    (Variables|Default|SetIsHooked false)))

(event EventActorBeginOverlap
  (params (OtherActor :type Actor%20Object%20Reference))
  (bind _returnvalue (Pawn|GetController))
  (bind _returnvalue_2 (Utilities|GetClass OtherActor))
  (bind _firsttarget (Variables|Default|GetFirstTarget))
  (bind _secondtarget (Variables|Default|GetSecondTarget))
  (if (Utilities|ClassIsChildOf _returnvalue_2 "/Script/WhatNow.Projectile")
    (Actor|DestroyActor)
    (elif (== OtherActor _firsttarget)
      (AI|Navigation|SimpleMovetoLocation _returnvalue (Transformation|GetActorLocation _secondtarget))
      (elif (== OtherActor _secondtarget)
        (AI|Navigation|SimpleMovetoLocation _returnvalue (Transformation|GetActorLocation _firsttarget))
        (elif (Utilities|ClassIsChildOf _returnvalue_2 "/Game/Blueprints/HookShot.HookShot_C")
          (bind _ashook_shot (Utilities|Casting|CastToHookShot OtherActor))
          (if (not (Variables|/Game/Blueprints/HookShot.HookShot_C|GetHasActor _ashook_shot))
            (Variables|Default|SetIsHooked true)
            (Variables|Default|SetHook _ashook_shot)
            (Variables|/Game/Blueprints/HookShot.HookShot_C|SetHasActor _ashook_shot true)))))))

(event EventTick
  (params (DeltaSeconds :type Float%20%28single-precision%29))
  (if (Variables|Default|GetIsHooked)
    (Transformation|SetActorLocation (Transformation|GetActorLocation (Variables|Default|GetHook)) false)))

(fn ConstructionScript
  (LocalVariables|SetCurrentTarget 0))