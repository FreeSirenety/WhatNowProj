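; Player character for a side-view game, locked to X = 0, that fires hook shots and respawns at checkpoints.
; Tick advances the shot cooldown and uses paired DoOnce nodes to turn touch state into IsTouching; BeginPlay adds a widget.
; Shoot spawns a scaled HookShot with sideways velocity based on facing; its ShotType switch has no distinct behavior.
; Overlapping a Checkpoint saves it, while touching a MyCharacter2 calls Die, which teleports back there.
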(event EventActorBeginOverlap
  (params (OtherActor :type Actor%20Object%20Reference))
  (bind _returnvalue (Utilities|GetClass OtherActor))
  (if (Utilities|ClassIsChildOf _returnvalue "/Game/Blueprints/MyCharacter2.MyCharacter2_C")
    (CallFunction|Die)
    (elif (Utilities|ClassIsChildOf _returnvalue "/Game/Blueprints/Checkpoint.Checkpoint_C")
      (bind _ascheckpoint (Utilities|Casting|CastToCheckpoint OtherActor))
      (Variables|Default|SetLastCheckPoint _ascheckpoint))))

(event EventTick
  (params (DeltaSeconds :type Float%20%28single-precision%29))
  (bind _returnvalue (Transformation|GetActorLocation))
  (bind (_x _y _z) (Math|Vector|BreakVector _returnvalue))
  (Variables|Default|SetHookShotTimer (+ (Variables|Default|GetHookShotTimer) DeltaSeconds))
  (Transformation|SetActorLocation (Math|Vector|MakeVector 0.0 _y _z) false)
  (bind _asplayer_controller (Utilities|Casting|CastToPlayerController (Pawn|GetController)))
  (if (.bIsCurrentlyPressed (Class|PlayerController|GetInputTouchState _asplayer_controller "Touch1"))
    (Utilities|FlowControl|DoOnce false :!label _label
      (:Completed
        (Utilities|FlowControl|Sequence
          (:then_0
            (Variables|Default|SetIsTouching true))
          (:then_1
            (goto _label_2 Reset)))))
    (else
      (Utilities|FlowControl|DoOnce false :!label _label_2
        (:Completed
          (Utilities|FlowControl|Sequence
            (:then_0
              (Variables|Default|SetIsTouching false))
            (:then_1
              (goto _label Reset))))))))

(event EventBeginPlay
  (bind _returnvalue (UserInterface|CreateWidget "/Game/NewWidgetBlueprint.NewWidgetBlueprint_C"))
  (UserInterface|Viewport|AddtoViewport _returnvalue))

(fn ConstructionScript
  (Variables|Default|SetShotType "NewEnumerator0"))

(fn Shoot
  (switch Utilities|FlowControl|Switch|SwitchonShotTypes (Variables|Default|GetShotType)
    (:NewEnumerator0
      _)
    (:NewEnumerator1
      _)
    (:NewEnumerator2
      _))
  (if (< 1.0 (Variables|Default|GetHookShotTimer))
    (Variables|Default|SetHookShotTimer 0.0)
    (bind _returnvalue (Game|SpawnActorfromClass "/Game/Blueprints/HookShot.HookShot_C" (Transformation|GetActorTransform) true 0))
    (Variables|/Game/Blueprints/HookShot.HookShot_C|SetTravelTime _returnvalue 2.0)
    (Transformation|SetActorScale3D _returnvalue (Math|Vector|MakeVector 3.0 3.0 3.0))
    (Math|Float|CompareFloat (.X (Math|Vector|BreakVector (.Y (Math|Rotator|BreakRotIntoAxes (Transformation|GetActorRotation))))) 0.0
      (:>
        (Variables|/Game/Blueprints/HookShot.HookShot_C|SetMaxVelocity _returnvalue "0,-200.000000, 0"))
      (:<
        (Variables|/Game/Blueprints/HookShot.HookShot_C|SetMaxVelocity _returnvalue "0,200.000000, 0")))))

(fn Die
  (Transformation|SetActorLocation (Transformation|GetActorLocation (Variables|Default|GetLastCheckPoint)) false))