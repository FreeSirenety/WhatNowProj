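; HookShot is a projectile actor that flies out, reverses and finally removes a grabbed enemy for a point.
; Tick moves it without sweep, scaling MaxVelocity by a pi-multiplied linear time ramp that slows, then reverses it.
; At 1.5 times TravelTime it unhooks GrabbedEnemy, orders it toward its FirstTarget, increments player Score, then destroys both actors.
; No hit detection or GrabbedEnemy assignment occurs here.
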(event EventTick
  (params (DeltaSeconds :type Float%20%28single-precision%29))
  (bind _traveltime (Variables|Default|GetTravelTime))
  (bind _grabbedenemy (Variables|Default|GetGrabbedEnemy))
  (Variables|Default|SetCurrentTimeTraveled (+ DeltaSeconds (Variables|Default|GetCurrentTimeTraveled)))
  (Transformation|SetActorLocation (+ (Transformation|GetActorLocation) (* (* (Variables|Default|GetMaxVelocity) (Math|Float|MultiplybyPi (- (/ (- _traveltime (Variables|Default|GetCurrentTimeTraveled)) (/ _traveltime 2.0)) 1.0))) DeltaSeconds)) false)
  (if (not (< (Variables|Default|GetCurrentTimeTraveled) (* _traveltime 1.5)))
    (Variables|/Game/Blueprints/MyCharacter2.MyCharacter2_C|SetIsHooked _grabbedenemy false)
    (AI|Navigation|SimpleMovetoLocation (Pawn|GetController _grabbedenemy) (Transformation|GetActorLocation (Variables|/Script/WhatNow.Enemy|GetFirstTarget _grabbedenemy)))
    (bind _asmy_character (Utilities|Casting|CastToMyCharacter (Game|GetPlayerCharacter 0)))
    (Variables|/Game/Blueprints/MyCharacter.MyCharacter_C|SetScore _asmy_character (+ 1 (Variables|/Game/Blueprints/MyCharacter.MyCharacter_C|GetScore _asmy_character)))
    (Actor|DestroyActor _grabbedenemy)
    (Actor|DestroyActor)))

(event EventBeginPlay
  (Variables|Default|SetStartPosition (Transformation|GetActorLocation)))

(fn ConstructionScript
  (Variables|Default|SetHasActor false))